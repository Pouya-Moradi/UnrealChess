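; BP_Player is the player's camera rig, framing the game from either a White or Black side.
; SetPlayerCamera eases the Azimuth pivot back to zero relative transform while gliding the Camera to the chosen side's marker component using MoveComponentTo.
; RotateCamera orbits the view by adding an axis value to Azimuth's yaw, zeroing pitch and roll.
; Initialize and the construction script are empty.
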(event Custom|SetPlayerCamera
  (params (Color :type EN_Color%20Enum :default "NewEnumerator0"))
  (bind _white (Variables|Default|GetWhite))
  (bind _black (Variables|Default|GetBlack))
  (bind _returnvalue (Transformation|GetRelativeTransform _black))
  (bind _returnvalue_2 (Transformation|GetRelativeTransform _white))
  (Components|MoveComponentTo (Variables|Default|GetAzimuth) "0, 0, 0" "0, 0, 0" true true 1.0 true)
  (switch Utilities|FlowControl|Switch|SwitchonEN_Color Color
    (:NewEnumerator0
      (Components|MoveComponentTo (Variables|Default|GetCamera) (.location _returnvalue_2) (.rotation _returnvalue_2) true true 3.0 true))
    (:NewEnumerator2
      (Components|MoveComponentTo (Variables|Default|GetCamera) (.location _returnvalue) (.rotation _returnvalue) true true 3.0 true))))

(fn ConstructionScript)

(fn Initialize)

(fn RotateCamera
  (params (Axis :type Float%20%28single-precision%29))
  (if true
    (Transformation|SetRelativeRotation (Variables|Default|GetAzimuth) (Math|Rotator|MakeRotator 0.0 0.0 (+ Axis (.yaw (Variables|/Script/Engine.SceneComponent|GetRelativeRotation (Variables|Default|GetAzimuth))))) false false)))